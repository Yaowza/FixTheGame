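; Potion pickup that increments the potion count of an overlapping BP_CustomTPS player and activates that player's pickup aura.
; On pickup it plays a sound, disables collision and swaps the potion's material.
; The FadeAndGlow timeline then drives emissive, opacity and the Popo effect's spawn rate, while a pickup effect activates and the minimap icon hides.
; The actor destroys itself after a short delay.
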(event `self.ReceiveBeginPlay`
  (`NiagaraComponent.SetVariableFloat` (`self.Popo`) "SpawnRate" (`self.base spawnrate`))
  (`SceneComponent.K2_SetWorldRotation` (`self.Icone_Minimap`) (struct :`Yaw` 90.0 :`Roll` -90.0) false false))

(event `self.ReceiveActorBeginOverlap`
  (params (OtherActor :type "Actor Object Reference"))
  (bind _asbp_custom_tps (cast `/Game/Blueprints/BP_CustomTPS` OtherActor))
  (set `/Game/Blueprints/BP_CustomTPS.PotionsNumber` (+ (`/Game/Blueprints/BP_CustomTPS.PotionsNumber` _asbp_custom_tps) 1.0) _asbp_custom_tps)
  (`ActorComponent.Activate` (`/Game/Blueprints/BP_CustomTPS.AuraPickUPPopo` _asbp_custom_tps) false)
  (`GameplayStatics.PlaySoundAtLocation` "/Game/Musics_and_SFX/SFX/Popo-pickup.Popo-pickup" (`self.K2_GetActorLocation`) (struct) 1.0 1.0 0.0 null null null null)
  (`PrimitiveComponent.SetCollisionResponseToAllChannels` (`self.SM_Potion_01`) "ECR_Ignore")
  (`PrimitiveComponent.SetCollisionResponseToAllChannels` (`self.Sphere`) "ECR_Ignore")
  (`PrimitiveComponent.SetMaterial` (`self.SM_Potion_01`) 0 "/Game/Assets/Dreamscape/Materials/Props/MI_Props_Potion_YOYO.MI_Props_Potion_YOYO")
  (`|ExecutionSequence`
    (:`then_0`
      (bind (_direction _glow _fade _spawn_rate) (`Timeline|fade and glow`)
        (:`Update`
          (`MeshComponent.SetScalarParameterValueOnMaterials` (`self.SM_Potion_01`) "Emissive Intensity" _glow)
          (`MeshComponent.SetScalarParameterValueOnMaterials` (`self.SM_Potion_01`) "opacity" _fade)
          (`NiagaraComponent.SetVariableFloat` (`self.Popo`) "SpawnRate" _spawn_rate))))
    (:`then_1`
      (`ActorComponent.Activate` (`self.Popopickup`) false)
      (`SceneComponent.SetHiddenInGame` (`self.Icone_Minimap`) true false)
      (`KismetSystemLibrary.Delay` 3.0)
      (`self.K2_DestroyActor`))))

(fn `UserConstructionScript`)