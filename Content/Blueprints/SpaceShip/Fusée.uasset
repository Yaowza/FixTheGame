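; Rocket actor that ends the game when the player interacts with it holding the required fuse count.
; Sphere overlap shows a camera-facing prompt widget and polls the player's interact flag through a Delay loop.
; A never-reset DoOnce checks the count: a mismatch briefly shows an error material and sound.
; A match disables input, plays the takeoff sequence with effects, shows the end widget and moves the player away.
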(event `self.ReceiveTick`
  (params (DeltaSeconds :type "Float (single-precision)"))
  (bind _widget (`self.Widget`))
  (bind _asbp_custom_tps (cast `/Game/Blueprints/BP_CustomTPS` (`GameplayStatics.GetPlayerPawn` 0)))
  (`SceneComponent.K2_SetWorldRotation` _widget (`KismetMathLibrary.FindLookAtRotation` (`SceneComponent.K2_GetComponentLocation` _widget) (`SceneComponent.K2_GetComponentLocation` (`/Game/Blueprints/BP_CustomTPS.Camera` _asbp_custom_tps))) false false))

(event `self.ReceiveActorBeginOverlap`
  (params (OtherActor :type "Actor Object Reference")))

(event `self.Sphere1.OnComponentBeginOverlap`
  (params (OverlappedComponent :type "PrimitiveComponent Object Reference") (OtherActor :type "Actor Object Reference") (OtherComp :type "PrimitiveComponent Object Reference") (OtherBodyIndex :type Integer) (bFromSweep :type Boolean) (SweepResult :type "HitResult Structure (by ref)"))
  (bind `_fuséeunreal` (`self.fuséeunreal`))
  (bind _asbp_custom_tps (cast `/Game/Blueprints/BP_CustomTPS` OtherActor))
  (set `self.playerin` true)
  (`SceneComponent.SetVisibility` (`self.Widget`) true false)
  (if (`self.playerin`) :!label _label
    (if (`/Game/Blueprints/BP_CustomTPS.Interracting ?` _asbp_custom_tps)
      (`/Engine/EditorBlueprintResources/StandardMacros.DoOnce` false
        (:`Completed`
          (if (== (`self.nombasfuse`) (`/Game/Blueprints/BP_CustomTPS.FuseCollected` _asbp_custom_tps))
            (`PrimitiveComponent.SetMaterial` `_fuséeunreal` 0 "/Game/Blueprints/SpaceShip/assezdefuse.assezdefuse")
            (set `self.finished` true)
            (`GameplayStatics.PlaySoundAtLocation` "/Game/Musics_and_SFX/Correct_Answer_Sound_Effect.Correct_Answer_Sound_Effect" (0.0 0.0 0.0) (struct) 1.0 1.0 0.0 null null null null)
            (`self.DisableInput` (`GameplayStatics.GetPlayerCharacter` 0) (`GameplayStatics.GetPlayerController` 0))
            (`KismetSystemLibrary.Delay` 2.0)
            (set `self.Playingcinématic` true)
            (`LevelSequencePlayer.CreateLevelSequencePlayer` "/Game/D2collageFin.D2collageFin" (make `MovieSceneSequencePlaybackSettings` true))
            (`PrimitiveComponent.SetMaterial` `_fuséeunreal` 0 "/Game/Blueprints/SpaceShip/Fuséeecompléter.Fuséeecompléter")
            (`GameplayStatics.SpawnSoundAttached` "/Game/Blueprints/SpaceShip/FuséeDécolage.FuséeDécolage" (`self.fuséeunreal`) "None" (0.0 0.0 0.0) (struct) "KeepRelativeOffset" false 1.0 1.0 0.0 null null)
            (`ActorComponent.Activate` (`self.feuuu1`) false)
            (bind _returnvalue (`|CreateWidget` "/Game/Blueprints/UI/WBP_Fin.WBP_Fin_C"))
            (`UserWidget.AddToViewport` _returnvalue 0)
            (bind _returnvalue_2 (`GameplayStatics.GetActorOfClass` "/Game/Blueprints/BP_CustomTPS.BP_CustomTPS_C"))
            (`self.K2_SetActorTransform` _returnvalue_2 (`KismetMathLibrary.MakeTransform` (10000.0 100000.0 10000.0)) false false)
            (else
              (`PrimitiveComponent.SetMaterial` `_fuséeunreal` 0 "/Game/Blueprints/SpaceShip/pasassezdefuse.pasassezdefuse")
              (`GameplayStatics.PlaySoundAtLocation` "/Game/Musics_and_SFX/Error_｜_Sound_Effects__No_Copyright_.Error_｜_Sound_Effects__No_Copyright_" (0.0 0.0 0.0) (struct) 1.0 1.0 0.0 null null null null)
              (`KismetSystemLibrary.Delay` 2.0)
              (`PrimitiveComponent.SetMaterial` `_fuséeunreal` 0 "/Game/Blueprints/SpaceShip/fuséenoncomplétée.fuséenoncomplétée")))))
      (else
        (`KismetSystemLibrary.Delay` 0.2)
        (goto _label)))))

(event `self.Sphere1.OnComponentEndOverlap`
  (params (OverlappedComponent :type "PrimitiveComponent Object Reference") (OtherActor :type "Actor Object Reference") (OtherComp :type "PrimitiveComponent Object Reference") (OtherBodyIndex :type Integer))
  (cast `/Game/Blueprints/BP_CustomTPS` OtherActor)
  (set `self.playerin` false)
  (`SceneComponent.SetVisibility` (`self.Widget`) false false))

(fn `UserConstructionScript`)