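; Collectible fuse pickup in the SpaceShip folder that tracks how many fuses exist and how many the player has collected.
; On BeginPlay, each fuse finds the Fusée actor, increments its Nombasfuse counter and prints the new total on screen.
; Overlap with a BP_CustomTPS character increments that character's FuseCollected count and destroys the fuse.
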(event `self.ReceiveBeginPlay`
  (bind _returnvalue (`GameplayStatics.GetActorOfClass` "/Game/Blueprints/SpaceShip/Fusée.Fusée_C"))
  (bind _output_get (set `/Game/Blueprints/SpaceShip/Fusée.nombasfuse` (+ (`/Game/Blueprints/SpaceShip/Fusée.nombasfuse` _returnvalue) 1.0) _returnvalue))
  (`KismetSystemLibrary.PrintString` (`KismetStringLibrary.Conv_DoubleToString` _output_get) true false (struct :`R` 1.0 :`B` 0.231228 :`A` 1.0) 20000.0))

(event `self.ReceiveActorBeginOverlap`
  (params (OtherActor :type "Actor Object Reference"))
  (bind _asbp_custom_tps (cast `/Game/Blueprints/BP_CustomTPS` OtherActor))
  (set `/Game/Blueprints/BP_CustomTPS.FuseCollected` (+ (`/Game/Blueprints/BP_CustomTPS.FuseCollected` _asbp_custom_tps) 1.0) _asbp_custom_tps)
  (`self.K2_DestroyActor`))

(event `self.ReceiveTick`
  (params (DeltaSeconds :type "Float (single-precision)")))

(fn `UserConstructionScript`)