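; Black hole actor that drags characters, physics props and projectiles toward its Singularité component and destroys them on contact.
; Tick sets velocity on every BP_Overwatchcharacter regardless of range, and on simulating StaticMeshActors inside Sphre.
; The projectile pull, additive and also bounded by Sphre, is nested in the mesh loop, so repeats per mesh.
; Sphere overlap toggles character capsule physics and collision, running a Delay-looped radial force while inside.
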(event `self.ReceiveTick`
  (params (DeltaSeconds :type "Float (single-precision)"))
  (bind _outactors (`GameplayStatics.GetAllActorsOfClass` "/Game/Overwatch3/FirstPerson/Blueprints/BP_Overwatchcharacter.BP_Overwatchcharacter_C"))
  (for _array_element _outactors
    (bind _returnvalue (`SceneComponent.K2_GetComponentLocation` (`Actor.RootComponent` _array_element)))
    (`PrimitiveComponent.SetPhysicsLinearVelocity` (`Character.CapsuleComponent` _array_element) (* (`KismetMathLibrary.GetForwardVector` (`KismetMathLibrary.FindLookAtRotation` _returnvalue (`SceneComponent.K2_GetComponentLocation` (`self.Singularité`)))) (`self.fze`)) false "None")
    (bind (_hitlocation _hitnormal _bonename _outhit _returnvalue_2) (`PrimitiveComponent.K2_SphereOverlapComponent` (`self.Singularité`) _returnvalue 0.0 true false false))
    (if _returnvalue_2
      (`self.K2_DestroyActor` _array_element))
    (bind _outactors_2 (`GameplayStatics.GetAllActorsOfClass` "/Script/Engine.StaticMeshActor"))
    (for _array_element_2 _outactors_2
      (if (`SceneComponent.IsSimulatingPhysics` (`Actor.RootComponent` _array_element_2) "None")
        (bind _returnvalue_3 (`SceneComponent.K2_GetComponentLocation` (`Actor.RootComponent` _array_element_2)))
        (bind (_hitlocation_2 _hitnormal_2 _bonename_2 _outhit_2 _returnvalue_4) (`PrimitiveComponent.K2_BoxOverlapComponent` :`self` (`self.Sphre`) :`InBoxCentre` _returnvalue_3))
        (if _returnvalue_4
          (`PrimitiveComponent.SetPhysicsLinearVelocity` (`StaticMeshActor.StaticMeshComponent` _array_element_2) (* (`KismetMathLibrary.GetForwardVector` (`KismetMathLibrary.FindLookAtRotation` _returnvalue_3 (`SceneComponent.K2_GetComponentLocation` (`self.Singularité`)))) (`self.fze`)) false "None")
          (bind (_hitlocation_3 _hitnormal_3 _bonename_3 _outhit_3 _returnvalue_5) (`PrimitiveComponent.K2_SphereOverlapComponent` (`self.Singularité`) _returnvalue_3 0.0 true false false))
          (if _returnvalue_5
            (`self.K2_DestroyActor` _array_element_2))
          (bind _outactors_3 (`GameplayStatics.GetAllActorsOfClass` "/Game/Overwatch3/FirstPerson/Blueprints/BP_FirstPersonProjectile.BP_FirstPersonProjectile_C" :!label _label))
          (for _array_element_3 _outactors_3
            (bind _returnvalue_6 (`SceneComponent.K2_GetComponentLocation` (`Actor.RootComponent` _array_element_3)))
            (bind (_hitlocation_4 _hitnormal_4 _bonename_4 _outhit_4 _returnvalue_7) (`PrimitiveComponent.K2_BoxOverlapComponent` :`self` (`self.Sphre`) :`InBoxCentre` _returnvalue_6))
            (if _returnvalue_7
              (`PrimitiveComponent.SetSimulatePhysics` (`/Game/Overwatch3/FirstPerson/Blueprints/BP_FirstPersonProjectile.CollisionComponent` _array_element_3) true)
              (`PrimitiveComponent.SetPhysicsLinearVelocity` (`/Game/Overwatch3/FirstPerson/Blueprints/BP_FirstPersonProjectile.CollisionComponent` _array_element_3) (* (`KismetMathLibrary.GetForwardVector` (`KismetMathLibrary.FindLookAtRotation` _returnvalue_6 (`SceneComponent.K2_GetComponentLocation` (`self.Singularité`)))) (`self.fze_projo`)) true "None")
              (bind (_hitlocation_5 _hitnormal_5 _bonename_5 _outhit_5 _returnvalue_8) (`PrimitiveComponent.K2_SphereOverlapComponent` (`self.Singularité`) _returnvalue_6 0.0 true false false))
              (if _returnvalue_8
                (`self.K2_DestroyActor` _array_element_3)))))
        (else
          (`|ExecutionSequence`
            (:`then_0`
              (goto _label))))))))

(event `self.Sphere.OnComponentBeginOverlap`
  (params (OverlappedComponent :type "PrimitiveComponent Object Reference") (OtherActor :type "Actor Object Reference") (OtherComp :type "PrimitiveComponent Object Reference") (OtherBodyIndex :type Integer) (bFromSweep :type Boolean) (SweepResult :type "HitResult Structure (by ref)"))
  (set `self.in ?` true)
  (bind _asbp_overwatchcharacter (cast `/Game/Overwatch3/FirstPerson/Blueprints/BP_Overwatchcharacter` OtherActor))
  (bind _capsulecomponent (`Character.CapsuleComponent` _asbp_overwatchcharacter))
  (`PrimitiveComponent.SetCollisionResponseToChannel` _capsulecomponent "ECC_WorldDynamic" "ECR_Overlap")
  (`PrimitiveComponent.SetSimulatePhysics` _capsulecomponent true)
  (if (`self.in ?`) :!label _label_2
    (`PrimitiveComponent.AddRadialForce` _capsulecomponent (`SceneComponent.K2_GetComponentLocation` (`self.Singularité`)) 5000.0 1.0 "RIF_Constant" true)
    (`PrimitiveComponent.AddRadialForce` OtherComp (`SceneComponent.K2_GetComponentLocation` (`self.Singularité`)) 5000.0 1.0 "RIF_Constant" true)
    (`KismetSystemLibrary.Delay` 1e-05)
    (goto _label_2)))

(event `self.Sphere.OnComponentEndOverlap`
  (params (OverlappedComponent :type "PrimitiveComponent Object Reference") (OtherActor :type "Actor Object Reference") (OtherComp :type "PrimitiveComponent Object Reference") (OtherBodyIndex :type Integer))
  (set `self.in ?` false)
  (bind _asbp_overwatchcharacter (cast `/Game/Overwatch3/FirstPerson/Blueprints/BP_Overwatchcharacter` OtherActor))
  (bind _capsulecomponent (`Character.CapsuleComponent` _asbp_overwatchcharacter))
  (`PrimitiveComponent.SetCollisionResponseToChannel` _capsulecomponent "ECC_WorldDynamic" "ECR_Block")
  (`PrimitiveComponent.SetSimulatePhysics` _capsulecomponent false))

(fn `UserConstructionScript`)