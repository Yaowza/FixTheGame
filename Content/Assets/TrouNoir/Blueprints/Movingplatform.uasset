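; Moving platform Blueprint that slides from its start position to a target point once the player steps on it.
; BeginPlay caches the Cube's world location and an EndLocation component's position.
; When BP_Genji2 overlaps the Playertoutch trigger, a timeline lerps the Cube between the two points without sweeping, with no reverse on exit.
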(event `self.ReceiveBeginPlay`
  (set `self.Start_loc` (`SceneComponent.K2_GetComponentLocation` (`self.Cube`)))
  (set `self.end_loc` (`SceneComponent.K2_GetComponentLocation` (`self.end location`))))

(event `self.playertoutch.OnComponentBeginOverlap`
  (params (OverlappedComponent :type "PrimitiveComponent Object Reference") (OtherActor :type "Actor Object Reference") (OtherComp :type "PrimitiveComponent Object Reference") (OtherBodyIndex :type Integer) (bFromSweep :type Boolean) (SweepResult :type "HitResult Structure (by ref)"))
  (cast `/Game/FirstPerson/Blueprints/BP_Genji2` OtherActor)
  (bind (_direction _newtrack_0) (`Timeline|Timeline_0`)
    (:`Update`
      (`SceneComponent.K2_SetWorldLocation` (`self.Cube`) (`KismetMathLibrary.VLerp` (`self.Start_loc`) (`self.end_loc`) _newtrack_0) false false))))

(fn `UserConstructionScript`)